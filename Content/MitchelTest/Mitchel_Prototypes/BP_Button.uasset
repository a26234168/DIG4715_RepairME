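; Prototype button that, when interacted with, starts a timed challenge that ends when a projectile hits its pop-up target.
; Interaction creates a timer widget and plays a StopWatch timeline, whose event track increments a counter shown as MM:SS.
; A valid hit during a run stops the timeline, shows the finish time on the widget and another text element, then hides the widget and clears the counter after a delay.
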(event OnComponentHit(Pop-Up)
  (params (HitComponent :type Primitive%20Component%20Object%20Reference) (OtherActor :type Actor%20Object%20Reference) (OtherComp :type Primitive%20Component%20Object%20Reference) (NormalImpulse :type Vector :default "0, 0, 0") (Hit :type Hit%20Result%20Structure%20%28by%20ref%29))
  ;[1 0.4843 0.6596] Stopping Timer
  (bind _asbp_projectile_base (Utilities|Casting|CastTo OtherActor))
  (Variables|Default|SetProjectile 0 _asbp_projectile_base)
  (if (Variables|Default|GetisRacing)
    (Utilities|FlowControl|Sequence
      (:then_0
        (CallFunction|END))
      (:then_1
        (CallFunction|Resetting)))))

(event Custom|Resetting
  ;[0.6878 1 0.987] Resetting Widget
  (if (Variables|Default|GetIsStop)
    (Utilities|FlowControl|Delay 1e+01)
    (Widget|SetVisibility (.Button_Timer (Variables|Default|GetButton_Timer)) "Hidden")
    (Variables|Default|SetTime 0.0)
    (Variables|Default|SetIsStop false)))

(event Custom|END
  ;[1 0.8562 0.5895] Adding "Finish Time:" to Widget
  (Rendering|Components|TextRender|SetText (Variables|Default|GetTimer (.Button_Timer (Variables|Default|GetButton_Timer))) (Utilities|Text|ToText(String) (Variables|Default|GetStopWatch_Value)))
  (bind _output_get (Variables|Default|SetCurrent%20Finish%20Time "Finish Time:"))
  (Rendering|Components|TextRender|SetText (Variables|Default|GetFinal_Time (.Button_Timer (Variables|Default|GetButton_Timer))) _output_get)
  ;[0.6245 1 0.5554] Saving Time for Level End
  (bind _output_get_2 (Variables|Default|SetPopUpFinishTime (Utilities|Text|ToText(String) (Utilities|String|Append "Pop-Up Target Time: " (Variables|Default|GetStopwatch_Value)))))
  (Rendering|Components|TextRender|SetText (Variables|Default|GetButton_FinalTimer) _output_get_2)
  (Variables|Default|SetisRacing false)
  (Variables|Default|SetisStop true)
  ;[1 1 1] Widget Text
  (Timeline|StopWatch Stop
    (:Update
      (Variables|Default|SetisTriggered true))
    (:StopWatch_Seconds
      (bind _result (Math|Float|IncrementFloat (Variables|Default|GetTime))
        (:%20%20
          (bind _output_get_3 (Variables|Default|SetStopWatch_Value (Utilities|String|Append (Utilities|String|Append (select (> (Math|Float|Floor (/ _result 6e+01)) 9) (Utilities|String|ToString(Integer) (Math|Float|Floor (/ _result 6e+01))) (Utilities|String|Append "0" (Utilities|String|ToString(Integer) (Math|Float|Floor (/ _result 6e+01))))) ":") (select (> (Math|Float|Floor (Math|Float|%(Float) _result 6e+01)) 9) (Utilities|String|ToString(Integer) (Math|Float|Floor (Math|Float|%(Float) _result 6e+01))) (Utilities|String|Append "0" (Utilities|String|ToString(Integer) (Math|Float|Floor (Math|Float|%(Float) _result 6e+01))))))))
          (Rendering|Components|TextRender|SetText (Variables|Default|GetTimer (.Button_Timer (Variables|Default|GetButton_Timer))) (Utilities|Text|ToText(String) _output_get_3)))))))

(event Custom|BPI_Interaction_1
  (Variables|Default|SetIsRacing true)
  (Variables|Default|SetIsStop false)
  (if (not (Variables|Default|GetIsTriggered))
    (Variables|Default|SetIsTriggered false)
    (Utilities|FlowControl|Sequence
      (:then_0
        ;[0.9199 0.5315 1] Create Reference to Player
        (bind _asbp_heavy_vehicle (Utilities|Casting|CastToClass)
          (:then
            (Variables|Default|SetReference 0 _asbp_heavy_vehicle)
            (bind _aslevel_timer (Utilities|Casting|CastTo (.Button_Timer (Variables|Default|GetButton_Timer))))
            (Variables|Default|SetTimer _aslevel_timer 0))
          (:CastFailed
            (Development|PrintString "Hello"))))
      (:then_1
        ;[0.4753 0.5506 1] Reference Widget
        (bind _returnvalue (UserInterface|CreateWidget 0 (Game|GetPlayerController 0)))
        (bind _output_get (Variables|Default|SetButton_Timer 0 _returnvalue))
        (UserInterface|Viewport|AddtoViewport _output_get 0))
      (:then_2
        ;[1 1 1] Widget Text
        (Timeline|StopWatch Play
          (:Update
            (Variables|Default|SetisTriggered true))
          (:StopWatch_Seconds
            (bind _result (Math|Float|IncrementFloat (Variables|Default|GetTime))
              (:%20%20
                (bind _output_get_2 (Variables|Default|SetStopWatch_Value (Utilities|String|Append (Utilities|String|Append (select (> (Math|Float|Floor (/ _result 6e+01)) 9) (Utilities|String|ToString(Integer) (Math|Float|Floor (/ _result 6e+01))) (Utilities|String|Append "0" (Utilities|String|ToString(Integer) (Math|Float|Floor (/ _result 6e+01))))) ":") (select (> (Math|Float|Floor (Math|Float|%(Float) _result 6e+01)) 9) (Utilities|String|ToString(Integer) (Math|Float|Floor (Math|Float|%(Float) _result 6e+01))) (Utilities|String|Append "0" (Utilities|String|ToString(Integer) (Math|Float|Floor (Math|Float|%(Float) _result 6e+01))))))))
                (Rendering|Components|TextRender|SetText (Variables|Default|GetTimer (.Button_Timer (Variables|Default|GetButton_Timer))) (Utilities|Text|ToText(String) _output_get_2))))))))))

(fn ConstructionScript)