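; Scene manager for the PNC toolkit's Overview scene, scripting its intro and example camera cutscenes.
; LoadStateFromStrings starts the intro from a saved state string; it blends to the player camera under opening credits with input disabled.
; Afterwards it restores input, clears that state, saves, and listens for one player action before unbinding.
; The example cutscene cuts between two timed cameras before blending back.
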(event Custom|OnActionPerformed
  (params (Actor :type Actor%20Object%20Reference) (Action :type EActions%20Enum :default "NewEnumerator11") (PlayAnim :type Boolean))
  ;[1 0.7494 0.4222 0.3] Disable the Move To tutorial notification when the action is performed.
  (if (Utilities|Enum|Equal(Enum) Action "NewEnumerator10")
    (EventDispatchers|UnbindEventfromActionPerformed (CallFunction|GetPNCPlayerController) (delegate Custom|OnActionPerformed))))

(event Custom|BeginIntroCutscene
  (if (CallFunction|IsCutsceneEnabled)
    ;[0.6084 1 0.8133 0.3] Disable player input, Play the intro cinematic, and add the opening credits to the players viewport.
    (Default|SetInputEnabled (CallFunction|GetPNCPlayerController) false)
    (Game|Player|SetViewTargetwithBlend (CallFunction|GetPNCPlayerController) (Variables|IntroCutscene|GetCutsceneCamera1) 0.0 "VTBlend_Linear" 0.0 false)
    (Game|Player|SetViewTargetwithBlend (CallFunction|GetPNCPlayerController) (CallFunction|GetPNCCameraManager) (Variables|IntroCutscene|GetCameraBlendTime) "VTBlend_Cubic" 5.0 false)
    (bind _returnvalue (UserInterface|CreateWidget "/Game/PNCTookit/PNCGame/Scenes/Shared/Widgets/WBP_OpeningCredits.WBP_OpeningCredits_C"))
    (UserInterface|Viewport|AddtoViewport _returnvalue 0)
    ;[0.6292 1 0.4586 0.3] After the camera has transitioned, reenable player input and setup the player/scene state for the first Movement tutorial.
    (Utilities|FlowControl|Delay (Variables|IntroCutscene|GetCameraBlendTime))
    (Default|SetInputEnabled (CallFunction|GetPNCPlayerController) true)
    (CallFunction|RemoveStateStringfromScene "" "MyFirstCutscene")
    (CallFunction|UserSaveGame)
    (EventDispatchers|BindEventtoActionPerformed (CallFunction|GetPNCPlayerController) (delegate Custom|OnActionPerformed))))

(event Custom|BeginExampleCutscene
  ;[1 1 1] Example Cutscene
  (Default|SetInputEnabled (CallFunction|GetPNCPlayerController) false)
  (Game|Player|SetViewTargetwithBlend (CallFunction|GetPNCPlayerController) (Variables|ExampleCutscene|GetExampleCutsceneCamera1) 0.0 "VTBlend_Linear" 0.0 false)
  (Utilities|FlowControl|Delay 3.0)
  (Game|Player|SetViewTargetwithBlend (CallFunction|GetPNCPlayerController) (Variables|ExampleCutscene|GetExampleCutsceneCamera2) 0.0 "VTBlend_Linear" 0.0 false)
  (Utilities|FlowControl|Delay 3.0)
  (Game|Player|SetViewTargetwithBlend (CallFunction|GetPNCPlayerController) (CallFunction|GetPNCCameraManager) 1.0 "VTBlend_EaseInOut" 5.0 false)
  (Default|SetInputEnabled (CallFunction|GetPNCPlayerController) true))

(fn ConstructionScript
  (|CallParentFunction))

(fn LoadStatefromStrings
  (for _array_element (Variables|Default|GetStateAsStrings)
    (switch string _array_element
      (:MyFirstCutscene
        (CallFunction|BeginIntroCutscene))))
  (return true))