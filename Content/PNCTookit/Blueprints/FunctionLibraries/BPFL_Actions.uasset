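; Blueprint function library for the point-and-click toolkit that decides which actions the player can perform on an actor.
; GetContextSensitiveActions gathers actions from interfaces and a door cast, then removes those disabled by the actor's GlobalInteractionComponent.
; GetContextSensitiveAction picks one action by class through per-type filters, falling back to MoveTo.
; Helpers spawn the actions menu, project interaction positions to screen, and validate interaction range.
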(fn GetContextSensitiveActions
  (params (Actor :type Actor%20Object%20Reference) (WithinRange :type Boolean))
  (bind _actionsref (LocalVariables|GetActionsRef))
  (bind _output_get (LocalVariables|SetActorRef Actor))
  (LocalVariables|SetbWithinInteractionRange WithinRange)
  ;[0.3904 0.797 1 0.3] Creates a list of Actions from implimented interfaces
  (bind _enumvalue (|ForEachEActions)
    (:LoopBody
      (switch Utilities|FlowControl|Switch|SwitchonEActions _enumvalue
        (:NewEnumerator0
          (if (Utilities|DoesObjectImplementInterface (LocalVariables|GetActorRef) "/Game/PNCTookit/Blueprints/Interface/BPI_ItemInteractions.BPI_ItemInteractions_C") :!label _label
            (if (Utilities|Enum|NotEqual(Enum) (Filter|FilterItemAction (LocalVariables|GetActorRef) (LocalVariables|GetbWithinInteractionRange)) "NewEnumerator11")
              (Utilities|Array|AddUnique (LocalVariables|GetActionsRef) (Filter|FilterItemAction (LocalVariables|GetActorRef) (LocalVariables|GetbWithinInteractionRange))))))
        (:NewEnumerator1
          (goto _label))
        (:NewEnumerator2
          (if (Utilities|DoesObjectImplementInterface (LocalVariables|GetActorRef) "/Game/PNCTookit/Blueprints/Interface/BPI_ObjectInteractions.BPI_ObjectInteractions_C") :!label _label_2
            (Utilities|Array|AddUnique (LocalVariables|GetActionsRef) "NewEnumerator2")
            (Utilities|Array|AddUnique (LocalVariables|GetActionsRef) "NewEnumerator6")))
        (:NewEnumerator6
          (goto _label_2))
        (:NewEnumerator7
          (if (Utilities|DoesObjectImplementInterface (LocalVariables|GetActorRef) "/Game/PNCTookit/Blueprints/Interface/BPI_Dialogue.BPI_Dialogue_C")
            (Utilities|Array|AddUnique (LocalVariables|GetActionsRef) "NewEnumerator7")))
        (:NewEnumerator9
          (bind _asbp_door_base (Utilities|Casting|CastToBP_DoorBase (LocalVariables|GetActorRef)))
          (Utilities|Array|AddUnique (LocalVariables|GetActionsRef) (Filter|FilterDoorAction _asbp_door_base)))))
    (:then
      ;[0.3904 0.797 1 0.3] Removes any actions set as "Disabled" in the Global Interactions Component on the actor.
      (if (>= (Utilities|Array|Length (LocalVariables|GetActionsRef)) 1)
        (bind _arrayelement (Utilities|Array|ReverseforEachLoop _actionsref)
          (:LoopBody
            (if (Utilities|Array|ContainsItem (Variables|/Game/PNCTookit/Blueprints/Components/BP_GlobalInteractionComponent.BP_GlobalInteractionComponent_C|GetDisabledInteractions (Actor|GetComponentbyClass _output_get "/Game/PNCTookit/Blueprints/Components/BP_GlobalInteractionComponent.BP_GlobalInteractionComponent_C")) _arrayelement)
              (Utilities|Array|RemoveItem (LocalVariables|GetActionsRef) _arrayelement)))
          (:Completed
            (return _actionsref) ; Finally, returns all the valid actions for the actor
          ))
        (else
          (return _actionsref) ; Finally, returns all the valid actions for the actor
        )))))

(fn FilterItemAction
  (params (Actor :type Actor%20Object%20Reference) (WthinInteractableRange :type Boolean))
  ;[0.5015 0.7837 1 0.3] Function used to filter the actor type for any unique cases where the actor type may change how the player can interact with it.
  (bind _output_get (LocalVariables|SetActorRef Actor))
  (Utilities|Casting|CastToBP_ItemBase _output_get
    (:then
      (if WthinInteractableRange
        (LocalVariables|SetActionRef "NewEnumerator1")
        (else
          (LocalVariables|SetActionRef "NewEnumerator1"))))
    (:CastFailed
      (if (Utilities|Name|NotEqual(Name) (Variables|/Game/PNCTookit/Blueprints/BP_PNCPlayerController.BP_PNCPlayerController_C|GetSelectedItemInInventory (CallFunction|GetPNCPlayerController)) "None")
        (LocalVariables|SetActionRef "NewEnumerator0")
        (else
          (LocalVariables|SetActionRef "NewEnumerator1")))))
  (return (LocalVariables|GetActionRef)))

(fn FilterNPCAction
  (params (NPC :type BP%20PNC%20Character%20Parent%20Object%20Reference))
  ;[0.5015 0.7837 1 0.3] Function used to filter the actor type for any unique cases where the actor type may change how the player can interact with it.
  (bind _output_get (LocalVariables|SetAction_Ref "NewEnumerator7"))
  (return _output_get))

(fn FilterDoorAction
  (params (Door :type BP%20Door%20Base%20Object%20Reference))
  ;[0.5015 0.7837 1 0.3] Function used to filter the actor type for any unique cases where the actor type may change how the player can interact with it.
  (LocalVariables|SetDoorRef Door)
  (if (Variables|/Game/PNCTookit/Blueprints/Gameplay/Scene/BP_DoorBase.BP_DoorBase_C|GetbIsUnlocked (LocalVariables|GetDoorRef))
    _
    (else
      _))
  (LocalVariables|SetAction_Ref "NewEnumerator9")
  (return (LocalVariables|GetAction_Ref)))

(fn FilterInteractableObjectAction
  (params (InteractableObject :type BP%20Interactable%20Object%20Base%20Object%20Reference))
  ;[0.5015 0.7837 1 0.3] Function used to filter the actor type for any unique cases where the actor type may change how the player can interact with it.
  (LocalVariables|SetInteractableObject_Ref InteractableObject)
  (LocalVariables|SetAction_Ref "NewEnumerator2")
  (return (LocalVariables|GetAction_Ref)))

(fn ShowActionsMenuforActor
  (params (Actor :type Actor%20Object%20Reference))
  ;[0.5015 0.7837 1 0.3] Create and add a Actions menu to the screeen on top of the given actor
  (LocalVariables|SetActorRef Actor)
  (bind _returnvalue (UserInterface|CreateWidget "/Game/PNCTookit/Blueprints/Widgets/Gameplay/WBP_ActionsMenu.WBP_ActionsMenu_C"))
  (Default|InitMenu _returnvalue (LocalVariables|GetActorRef))
  (UserInterface|Viewport|AddtoViewport _returnvalue 8)
  (return _returnvalue))

(fn GetonScreenInteractionPosition
  (params (Actor :type Actor%20Object%20Reference))
  (bind _returnvalue (Actor|GetComponentbyClass Actor "/Game/PNCTookit/Blueprints/Components/BP_InteractionPositionComponent.BP_InteractionPositionComponent_C"))
  (bind _controller (CallFunction|GetPNCPlayerController))
  (bind _returnvalue_2 (Transformation|GetActorLocation Actor))
  (bind _controller_2 (CallFunction|GetPNCPlayerController))
  (bind _screenposition (Class|GameplayStatics|ProjectWorldtoScreen _controller_2 _returnvalue_2 false))
  (bind _returnvalue_3 (Transformation|GetWorldLocation _returnvalue))
  (bind _screenposition_2 (Class|GameplayStatics|ProjectWorldtoScreen _controller _returnvalue_3 false))
  ;[0.6277 1 0.5388 0.3] Return the projected "InteractionPostionComponents" world location to screen position
  ;
  ; If the Interaction Position COmponent doesnt exist on the actor, use the actors world location instead.
  (Utilities|IsValid Actor
    (:Is%20Valid
      (Utilities|IsValid _returnvalue
        (:Is%20Valid
          (return (Math|Vector2D|MakeVector2D (.x _screenposition_2) (.y _screenposition_2))))
        (:Is%20Not%20Valid
          (return (Math|Vector2D|MakeVector2D (.x _screenposition) (.y _screenposition))))))
    (:Is%20Not%20Valid
      (return ""))))

(fn GetContextSensitiveAction
  (params (Actor :type Actor%20Object%20Reference) (WithinRange :type Boolean))
  (LocalVariables|SetActorRef Actor)
  (LocalVariables|SetbWithinInteractionRange WithinRange)
  (Utilities|FlowControl|Sequence
    (:then_0
      ;[0.3851 1 0.9801 0.3] Is the actor an "Item"
      (bind _asbp_item_base (Utilities|Casting|CastToBP_ItemBase (LocalVariables|GetActorRef)))
      (LocalVariables|SetActionRef (Filter|FilterItemAction _asbp_item_base (LocalVariables|GetbWithinInteractionRange))))
    (:then_1
      ;[0.3851 1 0.9801 0.3] Is the actor a "NPC"
      (bind _asbp_pnccharacter_parent (Utilities|Casting|CastToBP_PNCCharacter_Parent (LocalVariables|GetActorRef)))
      (LocalVariables|SetActionRef (Filter|FilterNPCAction _asbp_pnccharacter_parent)))
    (:then_2
      ;[0.3851 1 0.9801 0.3] Is the actor a "Door"
      (bind _asbp_door_base (Utilities|Casting|CastToBP_DoorBase (LocalVariables|GetActorRef)))
      (LocalVariables|SetActionRef (Filter|FilterDoorAction _asbp_door_base)))
    (:then_3
      ;[0.3851 1 0.9801 0.3] Is the actor a "Interactable Object"
      (bind _asbp_interactable_object_base (Utilities|Casting|CastToBP_InteractableObjectBase (LocalVariables|GetActorRef))
        (:then
          (LocalVariables|SetActionRef (Filter|FilterInteractableObjectAction _asbp_interactable_object_base)))
        (:CastFailed
          (LocalVariables|SetActionRef "NewEnumerator10")))))
  (return (LocalVariables|GetActionRef)))

(fn IsInteractionValid
  (params (Actor%20A :type Actor%20Object%20Reference) (Actor%20B :type Actor%20Object%20Reference))
  (return (or (CallFunction|InteractionVolumeWithinRange Actor%20A Actor%20B) (CallFunction|ActorWithinRange Actor%20A Actor%20B 1.5e+02))))