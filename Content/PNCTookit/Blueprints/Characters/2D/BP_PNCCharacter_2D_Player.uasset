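; 2D player character for the PNC toolkit, which shows movement and actions through Paper2D flipbooks.
; Tick derives a look direction from velocity and switches between idle and directional walk animations; LookAt and TalkTo also update facing.
; PlaySpriteAnimation selects the flipbook, pausing movement for pickup and interact animations until they finish.
; Sprite mirroring by negative X scale is a temporary stand-in for directional sprites.
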(event Custom|AnimationDelays
  (params (Duration :type Float%20%28single-precision%29))
  ;[0.4135 1 0.8072 0.3] Set flipbook animation and character direction
  (CallFunction|SetMovementEnabled false)
  (Utilities|FlowControl|Delay Duration)
  (CallFunction|PlaySpriteAnimation (Variables|2DAnimation|GetCurrentAnimationState_0) true)
  (Variables|Default|SetbIsMovementEnabled true))

(event EventActionPerformed
  (params (Actor :type Actor%20Object%20Reference) (Action :type EActions%20Enum :default "NewEnumerator11") (PlayAnim :type Boolean))
  ;[0.739 0.8755 1 0.3] If the player performs an action, play the associated animation (If there is one)
  (CallFunction|OnActionPerformed Action Actor PlayAnim))

(event EventOnForceMoveComplete
  ;[1 0.5706 0.3575 0.3] When "On Force movement complete" is called, make sure the current animation has stopped
  (|CallParentFunction)
  (CallFunction|PlaySpriteAnimation "NewEnumerator1" false))

(event EventTick
  (params (DeltaSeconds :type Float%20%28single-precision%29))
  (|CallParentFunction DeltaSeconds)
  ;[0.4135 1 0.8072 0.3] Set flipbook animation and character direction
  (CallFunction|SetLookatDirection true "0, 0, 0" "NewEnumerator8")
  (if (Variables|Default|GetbIsMovementEnabled)
    (if (> (Math|Vector|VectorLength (Variables|/Script/Engine.MovementComponent|GetVelocity (Variables|Character|GetCharacterMovement))) 0.1)
      (CallFunction|PlaySpriteAnimation "NewEnumerator2" true)
      (else
        (CallFunction|PlaySpriteAnimation "NewEnumerator1" true)))))

(fn ConstructionScript
  (|CallParentFunction)
  (CallFunction|SetLookatDirection false "0, 0, 0" (Variables|System|GetLookAtDirection)))

(fn SetLookatDirection
  (params (bUseVelocityDirection :type Boolean) (ToLocation :type Vector) (ForceLookAtDirection :type EDirection%20Enum :default "NewEnumerator8"))
  (bind _returnvalue (Transformation|GetActorLocation))
  (bind _returnvalue_2 (Transformation|GetActorLocation))
  (bind _returnvalue_3 (Math|Vector|VectorLength ToLocation))
  (bind _returnvalue_4 (* 1.0 0.8))
  (bind _bincludediagonaldirectionalanimations (Variables|System|GetbIncludeDiagonalDirectionalAnimations))
  (bind _charactermovement (Variables|Character|GetCharacterMovement))
  (bind _returnvalue_5 (>= _returnvalue_3 0.1))
  (bind _returnvalue_6 (Math|Rotator|FindLookatRotation _returnvalue ToLocation))
  (bind _velocity (Variables|/Script/Engine.MovementComponent|GetVelocity _charactermovement))
  (bind _returnvalue_7 (+ _returnvalue_2 _velocity))
  (bind _returnvalue_8 (Math|Rotator|FindLookatRotation _returnvalue_2 _returnvalue_7))
  (bind _returnvalue_9 (select _returnvalue_5 _returnvalue_6 _returnvalue_8))
  (bind (_returnvalue_10 _returnrotation) (CallFunction|Get2DLookatDirection _returnvalue_9 _bincludediagonaldirectionalanimations))
  (if bUseVelocityDirection
    (if (>= (Math|Vector|VectorLength _velocity) 1.0) :!label _label ; Is the players movement velocity large enough to calculate a change in direction?
      (if (Utilities|Enum|NotEqual(Enum) (Variables|System|GetLookAtDirection) _returnvalue_10) :!label _label_2 ; Does the current movement direction NOT equal the newly calculate direction?
        (Variables|System|SetLookAtDirection _returnvalue_10)
        ;[1 1 1] TEMP - Will be replaced with sprites and no character flipping
        (if (Math|Boolean|ORBoolean (Utilities|Enum|Equal(Enum) (Variables|System|GetLookAtDirection) "NewEnumerator0") (Utilities|Enum|Equal(Enum) (Variables|System|GetLookAtDirection) "NewEnumerator2") (Utilities|Enum|Equal(Enum) (Variables|System|GetLookAtDirection) "NewEnumerator5") (Utilities|Enum|Equal(Enum) (Variables|System|GetLookAtDirection) "NewEnumerator7")) :!label _label_3
          (Transformation|SetRelativeScale3D (Variables|Default|GetPaperFlipbook) (Math|Conversions|ToVector(Float) _returnvalue_4))
          (elif (Math|Boolean|ORBoolean (Utilities|Enum|Equal(Enum) (Variables|System|GetLookAtDirection) "NewEnumerator3") (Utilities|Enum|Equal(Enum) (Variables|System|GetLookAtDirection) "NewEnumerator1") (Utilities|Enum|Equal(Enum) (Variables|System|GetLookAtDirection) "NewEnumerator4") (Utilities|Enum|Equal(Enum) (Variables|System|GetLookAtDirection) "NewEnumerator6"))
            (Transformation|SetRelativeScale3D (Variables|Default|GetPaperFlipbook) (Math|Vector|MakeVector (* _returnvalue_4 -1.0) _returnvalue_4 _returnvalue_4)))))
      (elif _returnvalue_5
        (goto _label_2)))
    (elif (Utilities|Enum|Equal(Enum) ForceLookAtDirection "NewEnumerator8")
      (goto _label)
      (else
        (Variables|System|SetLookAtDirection ForceLookAtDirection)
        (goto _label_3)))))

(fn PlaySpriteAnimation
  (params (Anim :type ECharacterAnimation%20Enum :default "NewEnumerator0") (bLooping :type Boolean))
  (bind _2danimation_idle_left (Variables|2DAnimation|Idle|Get2DAnimation_Idle_Left))
  (bind _2danimation_pickup (Variables|2DAnimation|Pickup|Get2DAnimation_Pickup))
  (bind _output_get (Variables|2DAnimation|SetbSpriteAnimationLooping bLooping))
  (if _output_get ; Is the animation Looping? If not, then disable movement while the animation plays
    (Variables|2DAnimation|SetCurrentAnimationState_0 Anim))
  (LocalVariables|SetPlay2DAnimation Anim)
  (switch Utilities|FlowControl|Switch|SwitchonECharacterAnimation (LocalVariables|GetPlay2DAnimation)
    (:NewEnumerator0
      ;[1 0.7766 0.503 0.3] Idle Animation
      (Sprite|SetFlipbook (Variables|Default|GetPaperFlipbook) (Utilities|Select :Index (Variables|System|GetLookAtDirection) :NewEnumerator8 0 :NewEnumerator0 _2danimation_idle_left :NewEnumerator1 _2danimation_idle_left :NewEnumerator2 _2danimation_idle_left :NewEnumerator3 _2danimation_idle_left :NewEnumerator4 _2danimation_idle_left :NewEnumerator5 _2danimation_idle_left :NewEnumerator6 _2danimation_idle_left :NewEnumerator7 _2danimation_idle_left) :!label _label))
    (:NewEnumerator1
      (goto _label))
    (:NewEnumerator9
      (goto _label))
    (:NewEnumerator2
      ;[1 0.7766 0.503 0.3] Walk Animation
      (Sprite|SetFlipbook (Variables|Default|GetPaperFlipbook) (Utilities|Select :Index (Variables|System|GetLookAtDirection) :NewEnumerator8 0 :NewEnumerator0 (Variables|2DAnimation|Walk|Get2DAnimation_Walk_Up) :NewEnumerator1 (Variables|2DAnimation|Walk|Get2DAnimation_Walk_UpLeft) :NewEnumerator2 (Variables|2DAnimation|Walk|Get2DAnimation_Walk_UpRight) :NewEnumerator3 (Variables|2DAnimation|Walk|Get2DAnimation_Walk_Down) :NewEnumerator4 (Variables|2DAnimation|Walk|Get2DAnimation_Walk_DownLeft) :NewEnumerator5 (Variables|2DAnimation|Walk|Get2DAnimation_Walk_DownRight) :NewEnumerator6 (Variables|2DAnimation|Walk|Get2DAnimation_Walk_Left) :NewEnumerator7 (Variables|2DAnimation|Walk|Get2DAnimation_Walk_Right))))
    (:NewEnumerator6
      ;[1 0.7766 0.503 0.3] Pickup Animation
      (Sprite|SetFlipbook (Variables|Default|GetPaperFlipbook) (Utilities|Select :Index (Variables|System|GetLookAtDirection) :NewEnumerator8 0 :NewEnumerator0 _2danimation_pickup :NewEnumerator1 _2danimation_pickup :NewEnumerator2 _2danimation_pickup :NewEnumerator3 _2danimation_pickup :NewEnumerator4 _2danimation_pickup :NewEnumerator5 _2danimation_pickup :NewEnumerator6 _2danimation_pickup :NewEnumerator7 _2danimation_pickup) :!label _label_2)
      (CallFunction|AnimationDelays (Class|PaperFlipbookComponent|GetFlipbookLength (Variables|Default|GetPaperFlipbook))))
    (:NewEnumerator7
      (goto _label_2))
    (:NewEnumerator8
      ;[1 0.7766 0.503 0.3] Talking Animation
      (Sprite|SetFlipbook (Variables|Default|GetPaperFlipbook) (Variables|2DAnimation|Talking|Get2DAnimation_Talking)))))

(fn PlayAnimation
  (params (Anim :type ECharacterAnimation%20Enum :default "NewEnumerator0") (Looping :type Boolean) (CancelMovement :type Boolean))
  (CallFunction|PlaySpriteAnimation Anim Looping)
  (return true))

(fn Lookat
  (params (LookAtLocation :type Vector :default "0, 0, 0"))
  (CallFunction|SetLookatDirection false LookAtLocation "NewEnumerator8")
  (return true))

(fn Talkto
  (params (Instigator :type Actor%20Object%20Reference) (Dialogue :type Name :default "None"))
  (bind _success (|CallParentFunction Instigator Dialogue))
  (if _success
    (CallFunction|SetLookatDirection false (Transformation|GetActorLocation) "NewEnumerator8"))
  (return _success))